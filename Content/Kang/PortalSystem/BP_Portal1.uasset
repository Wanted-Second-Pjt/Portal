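; Linked portal actor that shows a recursive view through its partner and teleports the player between them.
; Each tick it captures from the partner's clip-planed camera at mirrored player-camera poses, deepest first, into a render target on its plane material.
; When an overlapping point crosses the plane front-to-back, player-tagged objects get remapped transform, velocity and control rotation, with a camera cut.
; The detect box lets BP_FirstPersonCharacter overlap a custom collision channel.
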(event OnComponentBeginOverlap(PortalPlane)
  (params (OverlappedComponent :type Primitive%20Component%20Object%20Reference) (OtherActor :type Actor%20Object%20Reference) (OtherComp :type Primitive%20Component%20Object%20Reference) (OtherBodyIndex :type Integer) (bFromSweep :type Boolean) (SweepResult :type Hit%20Result%20Structure%20%28by%20ref%29))
  (bind _asplayer_character (Utilities|Casting|CastToPlayerCharacter OtherActor)))

(event OnComponentEndOverlap(PlayerDetectBox)
  (params (OverlappedComponent :type Primitive%20Component%20Object%20Reference) (OtherActor :type Actor%20Object%20Reference) (OtherComp :type Primitive%20Component%20Object%20Reference) (OtherBodyIndex :type Integer))
  (bind _asbp_first_person_character (Utilities|Casting|CastToBP_FirstPersonCharacter OtherActor))
  (Collision|SetCollisionResponsetoChannel (Variables|/Script/Engine.Character|GetCapsuleComponent _asbp_first_person_character) "ECC_GameTraceChannel2" "ECR_Block"))

(event OnComponentBeginOverlap(PlayerDetectBox)
  (params (OverlappedComponent :type Primitive%20Component%20Object%20Reference) (OtherActor :type Actor%20Object%20Reference) (OtherComp :type Primitive%20Component%20Object%20Reference) (OtherBodyIndex :type Integer) (bFromSweep :type Boolean) (SweepResult :type Hit%20Result%20Structure%20%28by%20ref%29))
  (bind _asbp_first_person_character (Utilities|Casting|CastToBP_FirstPersonCharacter OtherActor))
  (Collision|SetCollisionResponsetoChannel (Variables|/Script/Engine.Character|GetCapsuleComponent _asbp_first_person_character) "ECC_GameTraceChannel2" "ECR_Overlap"))

(event OnComponentEndOverlap(PortalPlane)
  (params (OverlappedComponent :type Primitive%20Component%20Object%20Reference) (OtherActor :type Actor%20Object%20Reference) (OtherComp :type Primitive%20Component%20Object%20Reference) (OtherBodyIndex :type Integer))
  (bind _asplayer_character (Utilities|Casting|CastToPlayerCharacter OtherActor)))

(event EventBeginPlay
  (bind _asplayer_character (Utilities|Casting|CastToPlayerCharacter (Components|GetOwner (Game|GetPlayerController 0)))
    (:then
      (Variables|Default|SetPlayer _asplayer_character))
    (:CastFailed
      _))
  (CallFunction|InitBP)
  (CallFunction|SetClipPlaneBP))

(event Collision|EventActorBeginOverlap
  (params (OtherActor :type Actor%20Object%20Reference)))

(event EventTick
  (params (DeltaSeconds :type Float%20%28single-precision%29))
  (CallFunction|UpdateSceneCaptureRecursiveBP "0, 0, 0" "0, 0, 0")
  (CallFunction|ShouldTeleportBP))

(event EventSetClipPlane
  (CallFunction|SetClipPlaneBP))

(event EventInit
  (CallFunction|InitBP))

(event EventShouldTeleport
  (CallFunction|ShouldTeleportBP))

(event EventTeleport
  (CallFunction|TeleportBP))

(event EventUpdateSceneCaptureRecursive
  (params (Location :type Vector :default "0, 0, 0") (Rotation :type Rotator :default "0, 0, 0"))
  (CallFunction|UpdateSceneCaptureRecursiveBP Location Rotation))

(event EventPortalActivation
  (CallFunction|PortalActivationBP))

(event EventPortalDeactivation
  (CallFunction|PortalDeactivationBP))

(fn ConstructionScript)

(fn UpdateSceneCaptureBP
  (bind _returnvalue (Transformation|GetActorTransform))
  (bind _returnvalue_2 (Game|GetPlayerCameraManager 0))
  (bind _transformcomponent (Variables|/Script/Engine.PlayerCameraManager|GetTransformComponent _returnvalue_2))
  (bind _returnvalue_3 (Transformation|GetWorldRotation _transformcomponent))
  (bind (_x _y _z) (Math|Rotator|BreakRotIntoAxes _returnvalue_3))
  (Transformation|SetWorldLocationAndRotation (Variables|/Script/Portal.PortalPortal|GetPortalCamera (Variables|Default|GetLinkedPortal)) (Math|Transform|TransformLocation (Transformation|GetActorTransform (Variables|Default|GetLinkedPortal)) (Math|Transform|InverseTransformLocation (Math|Transform|MakeTransform (.location _returnvalue) (.rotation _returnvalue) (Math|Vector|MakeVector (* (.x (.scale _returnvalue)) -1.0) (* (.y (.scale _returnvalue)) -1.0) (.z (.scale _returnvalue)))) (Transformation|GetWorldLocation (Variables|/Script/Engine.PlayerCameraManager|GetTransformComponent (Game|GetPlayerCameraManager 0))))) (Math|Rotator|MakeRotationfromAxes (Math|Transform|TransformDirection (Transformation|GetActorTransform (Variables|Default|GetLinkedPortal)) (Math|Vector|MirrorVectorbyNormal (Math|Vector|MirrorVectorbyNormal (Math|Transform|InverseTransformDirection (Transformation|GetActorTransform) _x) "1.000000,0.000000,0.000000") "0.000000,1.000000,0.000000")) (Math|Transform|TransformDirection (Transformation|GetActorTransform (Variables|Default|GetLinkedPortal)) (Math|Vector|MirrorVectorbyNormal (Math|Vector|MirrorVectorbyNormal (Math|Transform|InverseTransformDirection (Transformation|GetActorTransform) _y) "1.000000,0.000000,0.000000") "0.000000,1.000000,0.000000")) (Math|Transform|TransformDirection (Transformation|GetActorTransform (Variables|Default|GetLinkedPortal)) (Math|Vector|MirrorVectorbyNormal (Math|Vector|MirrorVectorbyNormal (Math|Transform|InverseTransformDirection (Transformation|GetActorTransform) _z) "1.000000,0.000000,0.000000") "0.000000,1.000000,0.000000"))) false false))

(fn SetClipPlaneBP
  (bind _portalcamera (Variables|Default|GetPortalCamera))
  (Utilities|IsValid (Variables|Default|GetLinkedPortal)
    (:Is%20Valid
      (Variables|/Script/Engine.SceneCaptureComponent2D|SetbEnableClipPlane _portalcamera true)
      (bind _output_get (Variables|/Script/Engine.SceneCaptureComponent2D|SetClipPlaneBase _portalcamera (+ (Transformation|GetWorldLocation (Variables|Default|GetPortalPlane)) (* (Math|Vector|GetForwardVector (Variables|Default|GetForwardDirection)) 1.5))))
      (Variables|/Script/Engine.SceneCaptureComponent2D|SetClipPlaneNormal _portalcamera (Math|Vector|GetForwardVector (Variables|Default|GetForwardDirection)))
      (Game|SpawnActorfromClass "/Script/Engine.StaticMeshActor" (Math|Transform|MakeTransform _output_get "0, 0, 0" "1.000000,1.000000,1.000000") "AlwaysSpawn" "MultiplyWithRoot" 0 0))
    (:Is%20Not%20Valid
      (Development|PrintString "NOCLIP" true true "(R=0.000000,G=0.660000,B=1.000000,A=1.000000)" 2.0 "333"))))

(fn InitBP
  (bind _returnvalue (Viewport|GetViewportSize))
  (bind _offsetvalue (Variables|Default|GetOffsetValue))
  (bind _forwarddirection (Variables|Default|GetForwardDirection))
  (bind _returnvalue_2 (Math|Vector|GetForwardVector _forwarddirection))
  (bind _returnvalue_3 (* _returnvalue_2 _offsetvalue))
  (Components|Tick|SetTickGroup "TG_PostUpdateWork")
  (bind _returnvalue_4 (Rendering|Material|CreateDynamicMaterialInstance "/Game/Kang/PortalSystem/M_Portal.M_Portal" "None" "None" :!class /Script/Engine.KismetMaterialLibrary))
  (bind _output_get (Variables|Default|SetPortalMaterial _returnvalue_4))
  (Rendering|Material|SetMaterial (Variables|Default|GetPortalPlane) 0 _output_get)
  (bind _returnvalue_5 (Rendering|CreateRenderTarget2D (Math|Float|Truncate (.x _returnvalue)) (Math|Float|Truncate (.y _returnvalue)) "RTF_RGBA16f"))
  (bind _output_get_2 (Variables|Default|SetPortalRenderTarget _returnvalue_5))
  (Variables|/Script/Engine.Texture|SetMipGenSettings _output_get_2 "TMGS_NoMipmaps")
  (Variables|/Script/Engine.Texture|SetbUseNewMipFilter _returnvalue_5 true)
  (Rendering|Material|SetTextureParameterValue (Variables|Default|GetPortalMaterial) "Texture" _output_get_2)
  (Variables|/Script/Engine.SceneCaptureComponent2D|SetTextureTarget (Variables|/Script/Portal.PortalPortal|GetPortalCamera (Variables|Default|GetLinkedPortal)) (Variables|Default|GetPortalRenderTarget))
  (Rendering|Material|SetVectorParameterValue (Variables|Default|GetPortalMaterial) "OffsetDistance" (Math|Color|MakeColor (.x _returnvalue_3) (.y _returnvalue_3) (.z _returnvalue_3)) :!class /Script/Engine.MaterialInstanceDynamic))

(fn TeleportBP
  (bind _returnvalue (Game|GetPlayerController 0))
  (bind _returnvalue_2 (Game|GetPlayerCharacter 0))
  (bind _teleportobject (Variables|Default|GetTeleportObject))
  (bind _teleportobject_2 (Variables|Default|GetTeleportObject))
  (bind _returnvalue_3 (Pawn|GetControlRotation _returnvalue :!class /Script/Engine.Controller))
  (bind _returnvalue_4 (Transformation|GetActorTransform _teleportobject))
  (bind _returnvalue_5 (Pawn|GetMovementComponent _returnvalue_2))
  (bind _returnvalue_6 (CallFunction|UpdateRotationBP _returnvalue_3))
  (if (Actor|ActorHasTag _teleportobject_2 "Player")
    (Transformation|SetActorTransform _teleportobject_2 (Math|Transform|MakeTransform (CallFunction|UpdateLocationBP (.location _returnvalue_4)) (CallFunction|UpdateRotationBP (.rotation _returnvalue_4)) "1.000000,1.000000,1.000000") false true)
    (bind _newvelocity (CallFunction|UpdateVelocityBP (Variables|/Script/Engine.MovementComponent|GetVelocity _returnvalue_5)))
    (bind _output_get (Variables|/Script/Engine.MovementComponent|SetVelocity _returnvalue_5 _newvelocity))
    (if (Actor|ActorHasTag _teleportobject_2 "Player")
      (bind _asbp_player (Utilities|Casting|CastToBP_Player (Variables|Default|GetTeleportObject)))
      (Default|SmoothOrientation _asbp_player _returnvalue_6)
      (Pawn|SetControlRotation (Game|GetPlayerController 0) _returnvalue_6)
      (Class|PlayerCameraManager|SetGameCameraCutThisFrame (Game|GetPlayerCameraManager 0)))))

(fn ShouldTeleportBP
  (bind _returnvalue (Transformation|GetActorLocation))
  (bind _playerdetectbox (Variables|Default|GetPlayerDetectBox))
  (bind _forwarddirection (Variables|Default|GetForwardDirection))
  (bind _overlappingactors (Collision|GetOverlappingActors _playerdetectbox 0 :!class /Script/Engine.PrimitiveComponent))
  (bind _returnvalue_2 (Math|Vector|GetForwardVector _forwarddirection))
  (bind _output (Utilities|Array|Get(acopy) _overlappingactors))
  (Utilities|IsValid _output
    (:Is%20Valid
      (bind _output_get (Variables|Default|SetTeleportObject _output))
      (if (Utilities|String|Contains (Utilities|GetDisplayName _output_get) "character")
        (bind _return (CallFunction|IsPointCrossingPortalBP (Transformation|GetWorldLocation (Variables|/Script/Engine.PlayerCameraManager|GetTransformComponent (Game|GetPlayerCameraManager 0))) _returnvalue _returnvalue_2))
        (if _return
          (CallFunction|TeleportBP))
        (else
          (bind _return_2 (CallFunction|IsPointCrossingPortalBP (Transformation|GetActorLocation _output_get) _returnvalue _returnvalue_2))
          (if _return_2
            (CallFunction|TeleportBP)))))))

(fn IsPointCrossingPortalBP
  (params (Point :type Vector) (PortalLocation :type Vector) (PortalNormal :type Vector))
  (LocalVariables|SetIsInFront (>= (Math|Vector|DotProduct PortalNormal (- Point PortalLocation)) 0.0))
  (bind _output_get (LocalVariables|SetPortalPlane (Class|KismetMathLibrary|MakePlanefromPointandNormal PortalLocation PortalNormal)))
  (LocalVariables|SetIsInteract (.ReturnValue (Class|KismetMathLibrary|LinePlaneIntersection (Variables|Default|GetLastPosition) Point _output_get)))
  (LocalVariables|SetIsCrossing (Math|Boolean|ANDBoolean (LocalVariables|GetIsInteract) (not (LocalVariables|GetIsInFront)) (Variables|Default|GetLastInFront)))
  (Variables|Default|SetLastInFront (LocalVariables|GetIsInFront))
  (Variables|Default|SetLastPosition Point)
  (return (LocalVariables|GetIsCrossing)))

(fn UpdateLocationBP
  (params (OldLocation :type Vector))
  (bind _returnvalue (Transformation|GetActorTransform))
  ;[0.15 0.15 0.15 0.5] UpdateLocation
  (return (Math|Transform|TransformLocation (Transformation|GetActorTransform (Variables|Default|GetLinkedPortal)) (Math|Transform|InverseTransformLocation (Math|Transform|MakeTransform (.location _returnvalue) (.rotation _returnvalue) (Math|Vector|MakeVector (* (.x (.scale _returnvalue)) -1.0) (* (.y (.scale _returnvalue)) -1.0) (.z (.scale _returnvalue)))) OldLocation))))

(fn UpdateRotationBP
  (params (OldRotation :type Rotator))
  (bind _returnvalue (Transformation|GetActorTransform))
  (bind (_x _y _z) (Math|Rotator|GetAxes OldRotation))
  ;[0.15 0.15 0.15 0.5] UpdateRotation
  (return (Math|Rotator|MakeRotationfromAxes (Math|Transform|TransformDirection (Transformation|GetActorTransform (Variables|Default|GetLinkedPortal)) (Math|Vector|MirrorVectorbyNormal (Math|Vector|MirrorVectorbyNormal (Math|Transform|InverseTransformDirection _returnvalue _x) "1.000000,0.000000,0.000000") "0.000000,1.000000,0.000000")) (Math|Transform|TransformDirection (Transformation|GetActorTransform (Variables|Default|GetLinkedPortal)) (Math|Vector|MirrorVectorbyNormal (Math|Vector|MirrorVectorbyNormal (Math|Transform|InverseTransformDirection _returnvalue _y) "1.000000,0.000000,0.000000") "0.000000,1.000000,0.000000")) (Math|Transform|TransformDirection (Transformation|GetActorTransform (Variables|Default|GetLinkedPortal)) (Math|Vector|MirrorVectorbyNormal (Math|Vector|MirrorVectorbyNormal (Math|Transform|InverseTransformDirection _returnvalue _z) "1.000000,0.000000,0.000000") "0.000000,1.000000,0.000000")))))

(fn UpdateSceneCaptureRecursiveBP
  (params (Location :type Vector) (Rotation :type Rotator))
  (bind _returnvalue (Game|GetPlayerCameraManager 0))
  (bind _transformcomponent (Variables|/Script/Engine.PlayerCameraManager|GetTransformComponent _returnvalue))
  (bind _returnvalue_2 (Transformation|GetWorldTransform _transformcomponent))
  (if (== (Variables|Default|GetCurrentRecursion) 0)
    (LocalVariables|SetTempLocation (CallFunction|UpdateLocationBP (.location _returnvalue_2)))
    (LocalVariables|SetTempRotation (CallFunction|UpdateRotationBP (.rotation _returnvalue_2)))
    (Math|Integer|IncrementInt (Variables|Default|GetCurrentRecursion)
      (:%20%20
        (CallFunction|UpdateSceneCaptureRecursiveBP (LocalVariables|GetTempLocation) (LocalVariables|GetTempRotation))
        (Transformation|SetWorldLocationAndRotation (Variables|/Script/Portal.PortalPortal|GetPortalCamera (Variables|Default|GetLinkedPortal)) (LocalVariables|GetTempLocation) (LocalVariables|GetTempRotation) false false)
        (Rendering|SceneCapture|CaptureScene (Variables|/Script/Portal.PortalPortal|GetPortalCamera (Variables|Default|GetLinkedPortal)) :!class /Script/Engine.SceneCaptureComponent2D)
        (Variables|Default|SetCurrentRecursion 0)))
    (elif (< (Variables|Default|GetCurrentRecursion) (Variables|Default|GetMaxRecursion))
      (LocalVariables|SetTempLocation (CallFunction|UpdateLocationBP Location))
      (LocalVariables|SetTempRotation (CallFunction|UpdateRotationBP Rotation))
      (Math|Integer|IncrementInt (Variables|Default|GetCurrentRecursion)
        (:%20%20
          (CallFunction|UpdateSceneCaptureRecursiveBP (LocalVariables|GetTempLocation) (LocalVariables|GetTempRotation))
          (Transformation|SetWorldLocationAndRotation (Variables|/Script/Portal.PortalPortal|GetPortalCamera (Variables|Default|GetLinkedPortal)) (LocalVariables|GetTempLocation) (LocalVariables|GetTempRotation) false false)
          (Rendering|SceneCapture|CaptureScene (Variables|/Script/Portal.PortalPortal|GetPortalCamera (Variables|Default|GetLinkedPortal)) :!class /Script/Engine.SceneCaptureComponent2D)))
      (else
        (Transformation|SetWorldLocationAndRotation (Variables|/Script/Portal.PortalPortal|GetPortalCamera (Variables|Default|GetLinkedPortal)) (CallFunction|UpdateLocationBP Location) (CallFunction|UpdateRotationBP Rotation) false false)
        (Rendering|SetVisibility (Variables|Default|GetPortalPlane) false false)
        (Rendering|SceneCapture|CaptureScene (Variables|/Script/Portal.PortalPortal|GetPortalCamera (Variables|Default|GetLinkedPortal)) :!class /Script/Engine.SceneCaptureComponent2D)
        (Rendering|SetVisibility (Variables|Default|GetPortalPlane) true false)))))

(fn UpdateVelocityBP
  (params (OldVelocity :type Vector))
  (return (* (Math|Transform|TransformDirection (Transformation|GetActorTransform (Variables|Default|GetLinkedPortal)) (Math|Vector|MirrorVectorbyNormal (Math|Transform|InverseTransformDirection (Transformation|GetActorTransform) (Math|Vector|Normalize OldVelocity)) "1.000000,0.000000,0.000000")) (Math|Vector|VectorLength OldVelocity))))

(fn PortalActivationBP
  (Components|Activation|Activate (Variables|Transformation|GetRootComponent) false)
  (Rendering|SetActorHiddenInGame false)
  (Collision|SetActorEnableCollision true)
  (CallFunction|SetClipPlaneBP))

(fn PortalDeactivationBP
  (Components|Activation|Deactivate (Variables|Transformation|GetRootComponent))
  (Rendering|SetActorHiddenInGame true)
  (Collision|SetActorEnableCollision false))

(fn IsPointCrossingPortal
  (params (Point :type Vector :default "0, 0, 0") (PortalLocation :type Vector :default "0, 0, 0") (PortalNormal :type Vector :default "0, 0, 0"))
  (bind _return (CallFunction|IsPointCrossingPortalBP Point PortalLocation PortalNormal))
  (return _return))

(fn UpdateLocation
  (params (OldLocation :type Vector :default "0, 0, 0"))
  (return (CallFunction|UpdateLocationBP OldLocation)))

(fn UpdateRotation
  (params (OldRotation :type Rotator :default "0, 0, 0"))
  (return (CallFunction|UpdateRotationBP OldRotation)))

(fn UpdateVelocity
  (params (OldVelocity :type Vector :default "0, 0, 0"))
  (bind _newvelocity (CallFunction|UpdateVelocityBP OldVelocity))
  (return _newvelocity))